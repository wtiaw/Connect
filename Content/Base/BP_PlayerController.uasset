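; Base player controller that opens the main UI window at play start and puts input in UI-only mode.
; BeginPlay fills ItemsArrays with a hardcoded sequence of Items0 and Items1, then creates BP_MainWindow and adds it to the viewport.
; Tick prints the index and up/down button names of every entry in Lines as a per-frame on-screen debug readout.
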(event `self.ReceiveBeginPlay`
  (`WidgetBlueprintLibrary.SetInputMode_UIOnlyEx` self null)
  (`KismetArrayLibrary.Array_Add` (`self.ItemsArrays`) (`self.Items_1`))
  (`KismetArrayLibrary.Array_Add` (`self.ItemsArrays`) (`self.Items_0`))
  (`KismetArrayLibrary.Array_Add` (`self.ItemsArrays`) (`self.Items_0`))
  (`KismetArrayLibrary.Array_Add` (`self.ItemsArrays`) (`self.Items_0`))
  (`KismetArrayLibrary.Array_Add` (`self.ItemsArrays`) (`self.Items_0`))
  (`KismetArrayLibrary.Array_Add` (`self.ItemsArrays`) (`self.Items_0`))
  (`KismetArrayLibrary.Array_Add` (`self.ItemsArrays`) (`self.Items_1`))
  (bind _returnvalue (`|CreateWidget` "/Game/MainWindow/BP_MainWindow.BP_MainWindow_C" (`GameplayStatics.GetPlayerController` 0)))
  (`UserWidget.AddToViewport` _returnvalue 0))

(event `self.ReceiveTick`
  (params (DeltaSeconds :type "Float (single-precision)"))
  (for (_array_element _array_index) (`self.Lines`)
    (`KismetSystemLibrary.PrintString` (`KismetStringLibrary.Concat_StrStr` (`KismetStringLibrary.Concat_StrStr` (`KismetStringLibrary.Concat_StrStr` (`KismetStringLibrary.Conv_IntToString` _array_index) " ") (`KismetStringLibrary.Concat_StrStr` (`KismetSystemLibrary.GetDisplayName` (break `Line` _array_element)) " ")) (`KismetSystemLibrary.GetDisplayName` (`.DownButton` (break `Line` _array_element)))) true true (struct :`G` 0.66 :`B` 1.0 :`A` 1.0) 0.0)))

(fn `UserConstructionScript`)